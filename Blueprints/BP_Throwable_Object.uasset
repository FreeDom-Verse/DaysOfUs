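; Throwable object actor that damages actors tagged "Damageable" on contact.
; Each tick it runs a one-unit line trace along world X from its sphere detection point on the Visibility channel.
; A tagged hit applies fixed damage, plays a sword-hit camera shake and spawns a blood splat at the impact.
; Nothing limits repeat hits, and the component hit event is empty.
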(event `self.Sphere_Detection_Point.OnComponentHit`
  (params (HitComponent :type "PrimitiveComponent Object Reference") (OtherActor :type "Actor Object Reference") (OtherComp :type "PrimitiveComponent Object Reference") (NormalImpulse :type "Vector Structure") (Hit :type "HitResult Structure (by ref)")))

(event `self.ReceiveTick`
  (params (DeltaSeconds :type "Float (single-precision)"))
  (bind _sphere_detection_point (`self.Sphere_Detection_Point`))
  (bind (_returnvalue_x _returnvalue_y _returnvalue_z) (`KismetMathLibrary.BreakVector` (`SceneComponent.K2_GetComponentLocation` _sphere_detection_point)))
  (bind (_outhit _returnvalue) (`KismetSystemLibrary.LineTraceSingle` (`SceneComponent.K2_GetComponentLocation` _sphere_detection_point) (`KismetMathLibrary.MakeVector` (+ _returnvalue_x 1.0) _returnvalue_y _returnvalue_z) "TraceTypeQuery1"))
  (if _returnvalue
    (bind (_bblockinghit _binitialoverlap _time _distance _location _impactpoint _normal _impactnormal _physmat _hitactor) (`GameplayStatics.BreakHitResult` _outhit))
    (if (`self.ActorHasTag` _hitactor "Damageable")
      (`GameplayStatics.ApplyDamage` _hitactor 10.0)
      (`GameplayStatics.PlayWorldCameraShake` "/Game/Blueprints/BP_SwordHit_CameraShake.BP_SwordHit_CameraShake_C" _location 0.0 2000.0)
      (`GameplayStatics.SpawnEmitterAtLocation` "/Game/FXs/Particles/Blood/P_Blood_Splat_Cone.P_Blood_Splat_Cone" _location (`KismetMathLibrary.MakeRotFromXY` _normal _normal) (0.4 0.4 0.4) true "AutoRelease"))))

(fn `UserConstructionScript`)