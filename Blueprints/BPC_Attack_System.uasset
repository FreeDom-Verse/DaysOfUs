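; Character component for BP_ThirdPersonCharacter that runs a five-step melee combo of sword slashes, a kick and a jump attack.
; Attack input plays the montage for the current AttackIndex or buffers a press, which SwordAttackCombo uses to continue or reset the chain.
; A looping timer sphere-traces along the blade with a hit cooldown, alongside a separate single-point trace.
; Hits on "Damageable" actors apply damage, camera shake, sound and blood particles.
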(event `self.ReceiveBeginPlay`
  (bind _asbp_third_person_character (cast `/Game/ThirdPerson/Blueprints/BP_ThirdPersonCharacter` (`self.GetOwner`)))
  (set `self.Character BP` _asbp_third_person_character)
  (set `self.Character Mesh` (`Character.Mesh` _asbp_third_person_character)))

(event `Attack 1`
  ;[0.05127 0.05127 0.05127] Combo System
  ;;[0.2664 0.009721 0.01764] Attack 1
  (`/Engine/EditorBlueprintResources/StandardMacros.DoOnce` false :!label _label
    (:`Completed`
      (`KismetSystemLibrary.Delay` 0.1)
      (`|PlayMontage` (`self.Character Mesh`) "/Game/ThirdPerson/RPG_Zanem/Animations/Mixamo_Combat_System/0_1Sword_Slash_UE_Montage.0_1Sword_Slash_UE_Montage"
        (:`then`
          (set `self.Attack Index` 1)
          (goto _label :!via `Reset`))))))

(event `EnhancedInput|/Game/ThirdPerson/Input/Actions/IA_Attack`
  (params (ActionValue :type Boolean) (ElapsedSeconds :type "Float (double-precision)") (TriggeredSeconds :type "Float (double-precision)") (InputAction :type "InputAction Object Reference" :default "/Game/ThirdPerson/Input/Actions/IA_Attack.IA_Attack"))
  ;[0.05127 0.05127 0.05127] Combo System
  ;;[0.2664 0.009721 0.01764] Attack Input
  (:`Started`
    (if (`self.Can Attack?`)
      (`self.Sword Attack`)
      (`self.Start Sword Trace_`))))

(event `Attack 2`
  ;[0.05127 0.05127 0.05127] Combo System
  ;;[0.2664 0.009721 0.01764] Attack 2
  (`/Engine/EditorBlueprintResources/StandardMacros.DoOnce` false :!label _label_2
    (:`Completed`
      (`KismetSystemLibrary.Delay` 0.1)
      (`|PlayMontage` (`self.Character Mesh`) "/Game/ThirdPerson/RPG_Zanem/Animations/Mixamo_Combat_System/0_2Sword_Slash_3__UE_Montage.0_2Sword_Slash_3__UE_Montage"
        (:`then`
          (set `self.Attack Index` 2)
          (goto _label_2 :!via `Reset`))))))

(event `Sword Attack`
  ;[0.05127 0.05127 0.05127] Combo System
  ;;[0.2664 0.009721 0.01764] Sword Attack
  (if (`self.Is Attacking? `)
    (set `self.Save Attack?` true)
    (else
      (set `self.Is Attacking? ` true)
      (switch `int` (`self.Attack Index`) :!label _label_3
        (:`0`
          (`self.Attack 1`))
        (:`1`
          (`self.Attack 2`))
        (:`2`
          (`self.Attack 3`))
        (:`3`
          (`self.Attack 4`))
        (:`4`
          (`self.Attack 5`))))))

(event `Attack 3`
  ;[0.05127 0.05127 0.05127] Combo System
  ;;[0.2664 0.009721 0.01764] Attack 3 (Kick)
  (`/Engine/EditorBlueprintResources/StandardMacros.DoOnce` false :!label _label_4
    (:`Completed`
      (`KismetSystemLibrary.Delay` 0.1)
      (`|PlayMontage` (`self.Character Mesh`) "/Game/ThirdPerson/RPG_Zanem/Animations/Mixamo_Combat_System/Sword_kick_UE_Montage.Sword_kick_UE_Montage"
        (:`then`
          (set `self.Attack Index` 3)
          (goto _label_4 :!via `Reset`))))))

(event `Sword Attack Combo`
  ;[0.05127 0.05127 0.05127] Combo System
  ;;[0.2664 0.009721 0.01764] Combo Continue
  (if (`self.Save Attack?`)
    (set `self.Save Attack?` false)
    (goto _label_3)
    (else
      (`self.Stop Combo`))))

(event `Attack 4`
  ;[0.05127 0.05127 0.05127] Combo System
  ;;[0.2664 0.009721 0.01764] Attack 4
  (`/Engine/EditorBlueprintResources/StandardMacros.DoOnce` false :!label _label_5
    (:`Completed`
      (`KismetSystemLibrary.Delay` 0.1)
      (`|PlayMontage` (`self.Character Mesh`) "/Game/ThirdPerson/RPG_Zanem/Animations/Mixamo_Combat_System/0_4Sword_attack_Turn_3__UE_Montage.0_4Sword_attack_Turn_3__UE_Montage"
        (:`then`
          (set `self.Attack Index` 4)
          (goto _label_5 :!via `Reset`))))))

(event `Stop Combo`
  ;[0.05127 0.05127 0.05127] Combo System
  ;;[0.2664 0.009721 0.01764] Stop Combo / Attack
  (set `self.Is Attacking? ` false)
  (set `self.Attack Index` 0))

(event `Reset Attack Combat`
  ;[0.05127 0.05127 0.05127] Combo System
  ;;[0.2664 0.009721 0.01764] Stop Combo / Attack
  (`/Engine/EditorBlueprintResources/StandardMacros.IncrementInt` (`self.Attack Index`)))

(event `Attack 5`
  ;[0.05127 0.05127 0.05127] Combo System
  ;;[0.2664 0.009721 0.01764] Attack 5
  (`/Engine/EditorBlueprintResources/StandardMacros.DoOnce` false :!label _label_6
    (:`Completed`
      (`KismetSystemLibrary.Delay` 0.1)
      (`|PlayMontage` (`self.Character Mesh`) "/Game/ThirdPerson/RPG_Zanem/Animations/Mixamo_Combat_System/0_6Sword_Jump_attack_UE_Montage.0_6Sword_Jump_attack_UE_Montage"
        (:`then`
          (set `self.Attack Index` 5)
          (goto _label_6 :!via `Reset`))))))

(event `Start Sword Trace_`
  ;[0.3372 0.0319 0.03955] Sword Trace
  (bind _returnvalue (`KismetSystemLibrary.K2_SetTimerDelegate` (delegate `Start Sword Loop_`) 0.01 true))
  (set `self.SwordTraceLoop` _returnvalue))

(event `Sphere Trace`
  (bind _returnvalue (`SceneComponent.K2_GetComponentLocation` (`/Game/ThirdPerson/Blueprints/BP_ThirdPersonCharacter.Sphere Trace` (`self.Character BP`))))
  ;[0.2664 0.009721 0.01764] Sphere Trace
  (bind (_outhit _returnvalue_2) (`KismetSystemLibrary.SphereTraceSingle` :`Start` _returnvalue :`End` _returnvalue :`Radius` 25.0 :`TraceChannel` "TraceTypeQuery1" :`DrawDebugType` "ForDuration" :`DrawTime` 0.2))
  (if _returnvalue_2
    (bind (_bblockinghit _binitialoverlap _time _distance _location _impactpoint _normal _impactnormal _physmat _hitactor) (`GameplayStatics.BreakHitResult` _outhit))
    (if (`Actor.ActorHasTag` _hitactor "Damageable")
      (`GameplayStatics.ApplyDamage` _hitactor 10.0)
      (`GameplayStatics.PlayWorldCameraShake` "/Game/Blueprints/BP_SwordHit_CameraShake.BP_SwordHit_CameraShake_C" _location 0.0 2000.0)
      (`self.Play Sword Hit Sounds`)
      (`GameplayStatics.SpawnEmitterAtLocation` "/Game/FXs/Particles/Blood/P_Blood_Splat_Cone.P_Blood_Splat_Cone" _location (`KismetMathLibrary.MakeRotFromXY` _normal _normal) (0.4 0.4 0.4) true "AutoRelease"))))

(event `Start Sword Loop_`
  ;[0.3372 0.0319 0.03955] Sword Trace
  (bind (_outhit _returnvalue) (`KismetSystemLibrary.SphereTraceSingle` :`Start` (`SceneComponent.K2_GetComponentLocation` (`/Game/ThirdPerson/Blueprints/BP_ThirdPersonCharacter.Ninja_Lava_Sword_TopPoint` (`self.Character BP`))) :`End` (`SceneComponent.K2_GetComponentLocation` (`/Game/ThirdPerson/Blueprints/BP_ThirdPersonCharacter.Ninja_Lava_Sword_BottomPoint` (`self.Character BP`))) :`Radius` 5.0 :`TraceChannel` "TraceTypeQuery1" :`bTraceComplex` true :`DrawDebugType` "ForOneFrame" :`DrawTime` 0.1))
  (if _returnvalue
    (bind (_bblockinghit _binitialoverlap _time _distance _location _impactpoint _normal _impactnormal _physmat _hitactor) (`GameplayStatics.BreakHitResult` _outhit))
    (if (`Actor.ActorHasTag` _hitactor "Damageable")
      (`/Engine/EditorBlueprintResources/StandardMacros.DoOnce` false :!label _label_7
        (:`Completed`
          (`GameplayStatics.ApplyDamage` _hitactor 10.0)
          (`GameplayStatics.PlayWorldCameraShake` "/Game/Blueprints/BP_SwordHit_CameraShake.BP_SwordHit_CameraShake_C" _location 0.0 2000.0)
          (`self.Play Sword Hit Sounds`)
          (`GameplayStatics.SpawnEmitterAtLocation` "/Game/FXs/Particles/Blood/P_Blood_Splat_Cone.P_Blood_Splat_Cone" _location (`KismetMathLibrary.MakeRotFromXY` _normal _normal) (0.4 0.4 0.4) true "AutoRelease")
          (`KismetSystemLibrary.Delay` 0.5)
          (goto _label_7 :!via `Reset`))))))

(event `Stop Sword Trace_`
  ;[0.3372 0.0319 0.03955] Sword Trace
  (`KismetSystemLibrary.K2_ClearAndInvalidateTimerHandle` (`self.SwordTraceLoop`)))

(event `Play Sword Hit Sounds`
  ;[0.2664 0.009721 0.01764] Play Sword Hit Sounds
  (`GameplayStatics.PlaySoundAtLocation` "/Game/Audio-Sound/Sword_Hits/MS_SwordHit.MS_SwordHit" (`Actor.K2_GetActorLocation` (`self.GetOwner`)) (struct) 1.0 1.0 0.0 "/Game/Audio-Sound/SA_Charcater.SA_Charcater" null null null))