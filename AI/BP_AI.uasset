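; Enemy AI character that fights with a sword combo and can be stealth-assassinated from behind by the player.
; Attack feeds a five-step montage combo indexed by AttackIndex, with timer-looped or single sphere traces damaging "Damageable" actors.
; Damage plays hit reactions, launches the character and updates BPCPlayerState, ragdolling on death; assassination plays a victim montage, then delayed ragdoll.
; Health, assassinate and investigation widgets rotate toward the camera every tick.
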(event `self.ReceiveBeginPlay`
  (bind _aswb_dummy_health_bar (cast `/Game/UI/WB_DummyHealthBar` (`WidgetComponent.GetWidget` (`self.Health Bar Widget`))))
  (set `self.HealthBar UI` _aswb_dummy_health_bar))

(event `self.ReceiveTick`
  (params (DeltaSeconds :type "Float (single-precision)"))
  ;[0 0.05781 1 0.1216] [LM]Assassinate Widget (UI)
  (`SceneComponent.K2_SetWorldRotation` (`self.Assassinate Widget`) (`KismetMathLibrary.FindLookAtRotation` (`SceneComponent.K2_GetComponentLocation` (`self.Assassinate Widget`)) (`SceneComponent.K2_GetComponentLocation` (`Actor.RootComponent` (`GameplayStatics.GetPlayerCameraManager` 0)))) false false)
  (`SceneComponent.K2_SetWorldRotation` (`self.Health Bar Widget`) (`KismetMathLibrary.FindLookAtRotation` (`SceneComponent.K2_GetComponentLocation` (`self.Assassinate Widget`)) (`SceneComponent.K2_GetComponentLocation` (`Actor.RootComponent` (`GameplayStatics.GetPlayerCameraManager` 0)))) false false)
  (`SceneComponent.K2_SetWorldRotation` (`self.Investigation Widget `) (`KismetMathLibrary.FindLookAtRotation` (`SceneComponent.K2_GetComponentLocation` (`self.Assassinate Widget`)) (`SceneComponent.K2_GetComponentLocation` (`Actor.RootComponent` (`GameplayStatics.GetPlayerCameraManager` 0)))) false false))

(event `Ragdoll`
  ;[0 0.05781 1 0.1216] Ragdoll
  (`|ExecutionSequence`
    (:`then_0`
      (`KismetSystemLibrary.Delay` 2.5)
      (`PrimitiveComponent.SetSimulatePhysics` (`self.Mesh`) true))
    (:`then_1`
      (`KismetSystemLibrary.Delay` 1.7)
      (`GameplayStatics.PlaySoundAtLocation` "/Game/Audio-Sound/Groans-Grunts-Hits/Grunt2-death-pain.Grunt2-death-pain" (`self.K2_GetActorLocation`) (struct) 1.0 1.0 0.0 "/Game/Audio-Sound/SA_Charcater.SA_Charcater" null null null))))

(event `self.Assassination Radius.OnComponentBeginOverlap`
  (params (OverlappedComponent :type "PrimitiveComponent Object Reference") (OtherActor :type "Actor Object Reference") (OtherComp :type "PrimitiveComponent Object Reference") (OtherBodyIndex :type Integer) (bFromSweep :type Boolean) (SweepResult :type "HitResult Structure (by ref)"))
  ;[0 0.05781 1 0.1216] Assassinate Radius
  (cast `/Game/ThirdPerson/Blueprints/BP_ThirdPersonCharacter` OtherActor)
  (`SceneComponent.SetVisibility` (`self.Assassinate Widget`) true false))

(event `self.Assassination Radius.OnComponentEndOverlap`
  (params (OverlappedComponent :type "PrimitiveComponent Object Reference") (OtherActor :type "Actor Object Reference") (OtherComp :type "PrimitiveComponent Object Reference") (OtherBodyIndex :type Integer))
  ;[0 0.05781 1 0.1216] Assassinate Radius
  (cast `/Game/ThirdPerson/Blueprints/BP_ThirdPersonCharacter` OtherActor)
  (`SceneComponent.SetVisibility` (`self.Assassinate Widget`) true false))

(event `self.ReceiveAnyDamage`
  (params (Damage :type "Float (single-precision)") (DamageType :type "DamageType Object Reference") (InstigatedBy :type "Controller Object Reference") (DamageCauser :type "Actor Object Reference"))
  (`self.PlayAnimMontage` (`|GetArrayItem` (`self.HitAnims`) (`KismetMathLibrary.RandomIntegerInRange` 0 (- (`KismetArrayLibrary.Array_Length` (`self.HitAnims`)) 1))))
  (bind _asbp_third_person_character (cast `/Game/ThirdPerson/Blueprints/BP_ThirdPersonCharacter` (`GameplayStatics.GetPlayerCharacter` 0)))
  (`self.LaunchCharacter` (* (`KismetMathLibrary.GetForwardVector` (`self.K2_GetActorRotation` _asbp_third_person_character)) 700.0))
  (`GameplayStatics.PlaySoundAtLocation` "/Game/Audio-Sound/Groans-Grunts-Hits/Grunt2-death-pain.Grunt2-death-pain" (`self.K2_GetActorLocation`) (struct) 1.0 (`KismetMathLibrary.RandomFloatInRange` 1.3 1.2) 0.0 "/Game/Audio-Sound/SA_Charcater.SA_Charcater" null null null)
  (bind _is_player_dead_ (`/Game/Blueprints/BPC_PlayerState.Decrease Health` (`self.BPC_PlayerState`) Damage))
  (if _is_player_dead_
    (`PrimitiveComponent.SetCollisionObjectType` (`self.Mesh`) "ECC_PhysicsBody")
    (`PrimitiveComponent.SetSimulatePhysics` (`self.Mesh`) true)
    (`GameplayStatics.PlaySoundAtLocation` "/Game/Audio-Sound/Groans-Grunts-Hits/Grunt2-death-pain.Grunt2-death-pain" (`self.K2_GetActorLocation`) (struct) 1.0 1.0 0.0 "/Game/Audio-Sound/SA_Charcater.SA_Charcater" null null null)
    (`SceneComponent.SetVisibility` (`self.Health Bar Widget`) false false)))

(event `Start Sword Trace_`
  ;[0.3372 0.0319 0.03955] Sword Trace
  (bind _returnvalue (`KismetSystemLibrary.K2_SetTimerDelegate` (delegate `Start Sword Loop_`) 0.001 true))
  (set `self.SwordTraceLoop` _returnvalue))

(event `Attack 1`
  ;[0.4342 0.4072 0.02217] Combo System
  ;;[0.2664 0.009721 0.01764] Attack 1
  (`/Engine/EditorBlueprintResources/StandardMacros.DoOnce` false :!label _label
    (:`Completed`
      (`KismetSystemLibrary.Delay` 0.1)
      (`|PlayMontage` null "/Game/ThirdPerson/RPG_Zanem/Animations/Mixamo_Combat_System/0_1Sword_Slash_UE_Montage.0_1Sword_Slash_UE_Montage"
        (:`then`
          (set `self.Attack Index` 1)
          (goto _label :!via `Reset`))))))

(event `Sword Combo Call From BT_AI`
  ;[0.4342 0.4072 0.02217] Combo System
  ;;[0.2664 0.009721 0.01764] Attack Input
  (if (`self.Can Attack?`)
    (`self.Sword Attack`)))

(event `Start Sword Loop_`
  ;[0.3372 0.0319 0.03955] Sword Trace
  (bind (_outhit _returnvalue) (`KismetSystemLibrary.SphereTraceSingle` :`Start` (`SceneComponent.K2_GetComponentLocation` (`self.S_Katana__Sword_TopPoint`)) :`End` (`SceneComponent.K2_GetComponentLocation` (`self.S_Katana_Sword_BottomPoint`)) :`Radius` 10.0 :`TraceChannel` "TraceTypeQuery1" :`DrawDebugType` "ForDuration" :`DrawTime` 0.1))
  (if _returnvalue
    (bind (_bblockinghit _binitialoverlap _time _distance _location _impactpoint _normal _impactnormal _physmat _hitactor) (`GameplayStatics.BreakHitResult` _outhit))
    (if (`self.ActorHasTag` _hitactor "Damageable")
      (`/Engine/EditorBlueprintResources/StandardMacros.DoOnce` false :!label _label_2
        (:`Completed`
          (`GameplayStatics.ApplyDamage` _hitactor 10.0)
          (`GameplayStatics.PlayWorldCameraShake` "/Game/Blueprints/BP_SwordHit_CameraShake.BP_SwordHit_CameraShake_C" _location 0.0 2000.0)
          (`self.Play Sword Hit Sounds`)
          (`GameplayStatics.SpawnEmitterAtLocation` "/Game/FXs/Particles/Blood/P_Blood_Splat_Cone.P_Blood_Splat_Cone" _location (`KismetMathLibrary.MakeRotFromXY` _normal _normal) (0.4 0.4 0.4) true "AutoRelease")
          (`KismetSystemLibrary.Delay` 0.5)
          (goto _label_2 :!via `Reset`))))))

(event `Attack 2`
  ;[0.4342 0.4072 0.02217] Combo System
  ;;[0.2664 0.009721 0.01764] Attack 2
  (`/Engine/EditorBlueprintResources/StandardMacros.DoOnce` false :!label _label_3
    (:`Completed`
      (`KismetSystemLibrary.Delay` 0.1)
      (`|PlayMontage` (`self.Mesh`) "/Game/ThirdPerson/RPG_Zanem/Animations/Mixamo_Combat_System/0_2Sword_Slash_3__UE_Montage.0_2Sword_Slash_3__UE_Montage"
        (:`then`
          (set `self.Attack Index` 2)
          (goto _label_3 :!via `Reset`))))))

(event `Stop Sword Trace_`
  ;[0.3372 0.0319 0.03955] Sword Trace
  (`KismetSystemLibrary.K2_ClearAndInvalidateTimerHandle` (`self.SwordTraceLoop`)))

(event `Sword Attack`
  ;[0.4342 0.4072 0.02217] Combo System
  ;;[0.2664 0.009721 0.01764] Sword Attack
  (if (`self.Is Attacking?`)
    (set `self.Save Attack?` true)
    (else
      (set `self.Save Attack?` true)
      (switch `int` (`self.Attack Index`) :!label _label_4
        (:`0`
          (`self.Attack 1`))
        (:`1`
          (`self.Attack 2`))
        (:`2`
          (`self.Attack 3`))
        (:`3`
          (`self.Attack 4`))
        (:`4`
          (`self.Attack 5`))))))

(event `Play Sword Hit Sounds`
  ;[0.3372 0.0319 0.03955] Sword Trace
  ;;[0.2664 0.009721 0.01764] Play Sword Hit Sounds
  (`GameplayStatics.PlaySoundAtLocation` "/Game/Audio-Sound/Sword_Hits/MS_SwordHit.MS_SwordHit" (`self.K2_GetActorLocation` (`self.GetOwner`)) (struct) 1.0 1.0 0.0 "/Game/Audio-Sound/SA_Charcater.SA_Charcater" null null null))

(event `Attack 3`
  ;[0.4342 0.4072 0.02217] Combo System
  ;;[0.2664 0.009721 0.01764] Attack 3 (Kick)
  (`/Engine/EditorBlueprintResources/StandardMacros.DoOnce` false :!label _label_5
    (:`Completed`
      (`KismetSystemLibrary.Delay` 0.1)
      (`|PlayMontage` (`self.Mesh`) "/Game/ThirdPerson/RPG_Zanem/Animations/Mixamo_Combat_System/0_3Sword_attack_2__UE_Montage.0_3Sword_attack_2__UE_Montage"
        (:`then`
          (set `self.Attack Index` 3)
          (goto _label_5 :!via `Reset`))))))

(event `Sword Attack Combo`
  ;[0.4342 0.4072 0.02217] Combo System
  ;;[0.2664 0.009721 0.01764] Combo Continue
  (if (`self.Save Attack?`)
    (set `self.Save Attack?` false)
    (goto _label_4)
    (else
      (`self.Stop Combo`))))

(event `Sphere Trace`
  (bind _returnvalue (`SceneComponent.K2_GetComponentLocation` (`self.Sphere Trace Pose`)))
  ;[0.2664 0.009721 0.01764] Sphere Trace
  (bind (_outhit _returnvalue_2) (`KismetSystemLibrary.SphereTraceSingle` :`Start` _returnvalue :`End` _returnvalue :`Radius` 25.0 :`TraceChannel` "TraceTypeQuery1" :`DrawDebugType` "ForDuration" :`DrawTime` 0.2))
  (if _returnvalue_2
    (bind (_bblockinghit _binitialoverlap _time _distance _location _impactpoint _normal _impactnormal _physmat _hitactor) (`GameplayStatics.BreakHitResult` _outhit))
    (if (`self.ActorHasTag` _hitactor "Damageable")
      (`GameplayStatics.ApplyDamage` _hitactor 10.0)
      (`GameplayStatics.PlayWorldCameraShake` "/Game/Blueprints/BP_SwordHit_CameraShake.BP_SwordHit_CameraShake_C" _location 0.0 2000.0)
      (`self.Play Sword Hit Sounds`)
      (`GameplayStatics.SpawnEmitterAtLocation` "/Game/FXs/Particles/Blood/P_Blood_Splat_Cone.P_Blood_Splat_Cone" _location (`KismetMathLibrary.MakeRotFromXY` _normal _normal) (0.4 0.4 0.4) true "AutoRelease"))))

(event `Attack 4`
  ;[0.4342 0.4072 0.02217] Combo System
  ;;[0.2664 0.009721 0.01764] Attack 4
  (`/Engine/EditorBlueprintResources/StandardMacros.DoOnce` false :!label _label_6
    (:`Completed`
      (`KismetSystemLibrary.Delay` 0.1)
      (`|PlayMontage` (`self.Mesh`) "/Game/ThirdPerson/RPG_Zanem/Animations/Mixamo_Combat_System/Sword_kick_UE_Montage.Sword_kick_UE_Montage"
        (:`then`
          (set `self.Attack Index` 4)
          (goto _label_6 :!via `Reset`))))))

(event `Stop Combo`
  ;[0.4342 0.4072 0.02217] Combo System
  ;;[0.2664 0.009721 0.01764] Stop Combo / Attack
  (set `self.Save Attack?` false)
  (set `self.Attack Index` 0))

(event `Attack 5`
  ;[0.4342 0.4072 0.02217] Combo System
  ;;[0.2664 0.009721 0.01764] Attack 5
  (`/Engine/EditorBlueprintResources/StandardMacros.DoOnce` false :!label _label_7
    (:`Completed`
      (`KismetSystemLibrary.Delay` 0.1)
      (`|PlayMontage` (`self.Mesh`) "/Game/ThirdPerson/RPG_Zanem/Animations/Mixamo_Combat_System/0_5Sword_Slash_Down_4__UE_Montage.0_5Sword_Slash_Down_4__UE_Montage"
        (:`then`
          (set `self.Attack Index` 5)
          (goto _label_7 :!via `Reset`))))))

(event `Investigation icon`
  (bind _investigation_widget_ (`self.Investigation Widget `))
  (`KismetSystemLibrary.PrintString` "Investigating" true true (struct :`R` 0.604167 :`G` 0.266099 :`B` 0.02832 :`A` 1.0))
  (`/Engine/EditorBlueprintResources/StandardMacros.FlipFlop`
    (:`A`
      (`SceneComponent.SetVisibility` _investigation_widget_ true false))
    (:`B`
      (`SceneComponent.SetVisibility` _investigation_widget_ false false))))

(event `/Game/Targeting/BP_Targeting_Interface.DisplayLockedOnWidget`
  (params (Show_Widget :type Boolean))
  (`SceneComponent.SetVisibility` (`self.TargetLockedOn`) Show_Widget false))

(fn `Attack`
  (returns (`Animation Duration` :type "Float (double-precision)"))
  (`self.Sword Combo Call From BT_AI`)
  (return 0.6))

(fn `Stealth Back Assassin`
  (returns (`Reference Location` :type "Vector Structure") (`Assassin Rotation` :type "Rotator Structure"))
  (`self.PlayAnimMontage` "/Game/ThirdPerson/RPG_Zanem/Animations/Assassinations/UE5/Quinn_02_Paired_Knife_Stealth_KidneyAndNeck_Vic_Montage.Quinn_02_Paired_Knife_Stealth_KidneyAndNeck_Vic_Montage")
  (`self.Ragdoll`)
  (`SceneComponent.SetVisibility` (`self.Assassinate Widget`) false false)
  (return (`SceneComponent.K2_GetComponentLocation` (`self.Assassin Reference`)) (`self.K2_GetActorRotation`)))

(fn `UserConstructionScript`)